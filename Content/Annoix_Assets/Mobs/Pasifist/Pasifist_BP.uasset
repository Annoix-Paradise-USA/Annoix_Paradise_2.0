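; Passive golem mob that wanders the navmesh, takes damage and drops loot when killed.
; It loops between walking to a random reachable point and idling briefly, restarting only when a move succeeds.
; Tick updates a widget life bar and turns it toward the player camera.
; AnyDamage lowers clamped Life with a hit sound; at zero it plays another sound, spawns Loot1 at a downward trace hit with random yaw, then destroys itself.
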(event Custom|Random-move
  ;[1 1 1] Random-motion
  (Components|Animation|PlayAnimation (Variables|Character|GetMesh) "/Game/Annoix_Assets/NPC/Golem/Golem3_Walking.Golem3_Walking" true)
  (bind _randomlocation (Class|NavigationSystemV1|GetRandomLocationinNavigableRadius (Transformation|GetActorLocation) 5e+03 0 0))
  (AI|AIMoveTo self _randomlocation 0 5.0 false
    (:OnSuccess
      (Components|Animation|PlayAnimation (Variables|Character|GetMesh) "/Game/Annoix_Assets/NPC/Golem/Golem3_Idle.Golem3_Idle" true)
      (Utilities|FlowControl|Delay 5.0)
      (CallFunction|Random-move))))

(event Custom|Drop-Loot
  (bind _returnvalue (Transformation|GetActorLocation))
  ;[1 1 1] Drop loot enemy-Bp
  (bind _outhit (Collision|LineTraceByChannel _returnvalue (- _returnvalue "0,0,500.000000") "TraceTypeQuery1" false (Utilities|Array|MakeArray (Game|GetPlayerCharacter 0)) "None"))
  (Game|SpawnActorfromClass "/Game/Annoix_Assets/Props/Items/Loot-1.Loot-1_C" (Math|Transform|MakeTransform (.Location (Collision|BreakHitResult _outhit)) (Math|Rotator|MakeRotator 0.0 0.0 (Math|Random|RandomFloatinRange 0.0 3.6e+02))) "Undefined" 0 0))

(event Game|Damage|EventAnyDamage
  (params (Damage :type Float%20%28single-precision%29) (DamageType :type Damage%20Type%20Object%20Reference) (InstigatedBy :type Controller%20Object%20Reference) (DamageCauser :type Actor%20Object%20Reference))
  ;[1 1 1] Death
  (if (not (Variables|Default|GetIs%20Death))
    (bind _output_get (Variables|Default|Setlife (Math|Float|Clamp(Float) (- (Variables|Default|Getlife) Damage) 0.0 (Variables|Default|Getmax%20life))))
    (if (== _output_get 0.0)
      (Audio|PlaySound2D "/Game/Annoix_Assets/Sounds/SFX/Iniciar_campaña.Iniciar_campaña" 1.0 1.0 0.0 0 0)
      (Variables|Default|SetIs%20Death true)
      (CallFunction|Drop-Loot)
      (Actor|DestroyActor)
      (else
        (Audio|PlaySound2D "/Game/Annoix_Assets/Sounds/SFX/Hit_sword.Hit_sword" 1.0 1.0 0.0 0 0)))))

(event EventTick
  (params (DeltaSeconds :type Float%20%28single-precision%29))
  (bind _life_bar_widget (Variables|Default|Getlife-bar-widget))
  ;[1 1 1] LiVE-Bar
  (bind _asui_live_enemy (Utilities|Casting|CastToui-live-enemy (UserInterface|GetUserWidgetObject (Variables|Default|Getlife-bar-widget))))
  (Progress|SetPercent (Variables|/Game/Annoix_Assets/Interface/Dialogues/ui-live-enemy.ui-live-enemy_C|GetBar-life-enemy _asui_live_enemy) (/ (Variables|Default|Getlife) (Variables|Default|Getmax%20life)))
  (Transformation|SetWorldRotation _life_bar_widget (Math|Rotator|FindLookatRotation (Transformation|GetWorldLocation _life_bar_widget) (Transformation|GetWorldLocation (Variables|/Script/Engine.PlayerCameraManager|GetTransformComponent (Game|GetPlayerCameraManager 0)))) false false))

(event EventBeginPlay
  (CallFunction|Random-move))

(fn ConstructionScript)