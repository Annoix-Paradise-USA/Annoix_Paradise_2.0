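; ObjectiveBP is a one-shot trigger actor that hands Kazumi a new objective.
; On BeginPlay it casts its owner to ObjectiveButterBP and stores it as the paired mission actor.
; When KazumiCh_BP overlaps its Box, it sets the character's current objective, calls SlideOn and plays a new-mission sound.
; It then destroys itself and the paired ObjectiveButterBP.
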(event OnComponentBeginOverlap(Box)
  (params (OverlappedComponent :type Primitive%20Component%20Object%20Reference) (OtherActor :type Actor%20Object%20Reference) (OtherComp :type Primitive%20Component%20Object%20Reference) (OtherBodyIndex :type Integer) (bFromSweep :type Boolean) (SweepResult :type Hit%20Result%20Structure%20%28by%20ref%29))
  (bind _askazumi_ch_bp (Utilities|Casting|CastToKazumiCh_BP OtherActor))
  (Variables|/Game/Annoix_Assets/Character/Ch_Mechanics/KazumiCh_BP.KazumiCh_BP_C|SetCurrentObjective _askazumi_ch_bp (Variables|Default|GetObjective))
  (Default|Slideon _askazumi_ch_bp)
  (Audio|PlaySound2D "/Game/Annoix_Assets/Sounds/SFX/PresionaStart-Aceptar-NuevaMision.PresionaStart-Aceptar-NuevaMision" 1.0 1.0 0.0 0 0)
  (Actor|DestroyActor)
  (Actor|DestroyActor (Variables|Default|GetOtherMissionB)))

(event EventBeginPlay
  (bind _asobjective_butter_bp (Utilities|Casting|CastToObjectiveButterBP (Components|GetOwner)))
  (Variables|Default|SetOtherMissionB _asobjective_butter_bp))

(fn ConstructionScript)