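; Mission objective completion trigger for the ButterblyCh_BP character, paired with an owning ObjectiveCompletedBP actor that it caches on BeginPlay.
; When that character overlaps its Box and its CurrentObjective matches this Objective, it calls SlideOff on the character and plays a 2D sound.
; It then destroys both itself and the owning ObjectiveCompletedBP, removing both mission end points at once.
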(event OnComponentBeginOverlap(Box)
  (params (OverlappedComponent :type Primitive%20Component%20Object%20Reference) (OtherActor :type Actor%20Object%20Reference) (OtherComp :type Primitive%20Component%20Object%20Reference) (OtherBodyIndex :type Integer) (bFromSweep :type Boolean) (SweepResult :type Hit%20Result%20Structure%20%28by%20ref%29))
  (bind _asbutterbly_ch_bp (Utilities|Casting|CastToButterblyCh_BP OtherActor))
  (if (Utilities|Enum|Equal(Enum) (Variables|/Game/Annoix_Assets/Props/Vehicle/ButterblyCh_BP.ButterblyCh_BP_C|GetCurrentObjective _asbutterbly_ch_bp) (Variables|Default|GetObjective))
    (Default|SlideOff _asbutterbly_ch_bp)
    (Audio|PlaySound2D "/Game/Annoix_Assets/Sounds/SFX/Cancelar-Regresar.Cancelar-Regresar" 1.0 1.0 0.0 0 0)
    (Actor|DestroyActor)
    (Actor|DestroyActor (Variables|Default|GetOtherEndMissionA))))

(event EventBeginPlay
  (bind _asobjective_completed_bp (Utilities|Casting|CastToObjectiveCompletedBP (Components|GetOwner)))
  (Variables|Default|SetOtherEndMissionA _asobjective_completed_bp))

(fn ConstructionScript)