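; Mission objective trigger that hands its objective to the butterfly player character (ButterblyCh_BP) when that character overlaps its box.
; On overlap it sets the character's current objective, calls SlideOn and plays a new-mission sound.
; It then destroys itself along with the other mission actor, which BeginPlay takes from its owner cast to ObjectiveBP.
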(event OnComponentBeginOverlap(Box)
  (params (OverlappedComponent :type Primitive%20Component%20Object%20Reference) (OtherActor :type Actor%20Object%20Reference) (OtherComp :type Primitive%20Component%20Object%20Reference) (OtherBodyIndex :type Integer) (bFromSweep :type Boolean) (SweepResult :type Hit%20Result%20Structure%20%28by%20ref%29))
  (bind _asbutterbly_ch_bp (Utilities|Casting|CastToButterblyCh_BP OtherActor))
  (Variables|/Game/Annoix_Assets/Props/Vehicle/ButterblyCh_BP.ButterblyCh_BP_C|SetCurrentObjective _asbutterbly_ch_bp (Variables|Default|GetObjective))
  (Default|Slideon _asbutterbly_ch_bp)
  (Audio|PlaySound2D "/Game/Annoix_Assets/Sounds/SFX/PresionaStart-Aceptar-NuevaMision.PresionaStart-Aceptar-NuevaMision" 1.0 1.0 0.0 0 0)
  (Actor|DestroyActor)
  (Actor|DestroyActor (Variables|Default|GetOtherMissionA)))

(event EventBeginPlay
  (bind _asobjective_bp (Utilities|Casting|CastToObjectiveBP (Components|GetOwner)))
  (Variables|Default|SetOtherMissionA _asobjective_bp))

(fn ConstructionScript)